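; BP_AI_ExplosiveEnemy_Child is a suicide-style enemy that explodes on contact with the Ouroboros player or any BP_Bodies actor.
; DamageCapsule overlap drives everything: either contact damages the player, then spawns a Niagara burst and plays an explosion sound.
; It then decrements the game mode's enemy count and destroys itself.
; Other overlaps only print the actor's name, and construction defers to the parent.
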(event `self.DamageCapsule.OnComponentBeginOverlap`
  (params (OverlappedComponent :type "PrimitiveComponent Object Reference") (OtherActor :type "Actor Object Reference") (OtherComp :type "PrimitiveComponent Object Reference") (OtherBodyIndex :type Integer) (bFromSweep :type Boolean) (SweepResult :type "HitResult Structure (by ref)"))
  (bind _asgame_mode_ouroboros (`/Game/CORE/FL_Macro.GetGameModeOuroboros`))
  (if (== OtherActor (`/Game/CORE/FL_Macro.GetPlayerOuroboros`))
    (`GameplayStatics.ApplyDamage` (`/Game/CORE/FL_Macro.GetPlayerOuroboros`) (`self.Damage`) null self :!label _label)
    (`NiagaraFunctionLibrary.SpawnSystemAtLocation` "/Game/CORE/VFX/NB_TailDestroy1.NB_TailDestroy1" (`SceneComponent.K2_GetComponentLocation` (`self.CapsuleComponent`)))
    (`GameplayStatics.PlaySound2D` "/Game/CORE/Sound/SFX/SC_Explosion.SC_Explosion" 1.0 1.0 0.0 null null)
    (set `/Game/CORE/Game_Mode_Ouroboros.ActualNumberEnnemies` (- (`/Game/CORE/Game_Mode_Ouroboros.ActualNumberEnnemies` _asgame_mode_ouroboros) 1.0) _asgame_mode_ouroboros)
    (`KismetSystemLibrary.PrintString` "BOOM BOOM BOOM !")
    (`self.K2_DestroyActor`)
    (else
      (cast `/Game/CORE/BP/BP_Bodies` OtherActor
        (:`then`
          (goto _label))
        (:`CastFailed`
          (`KismetSystemLibrary.PrintString` (`KismetSystemLibrary.GetDisplayName` OtherActor)))))))

(fn `UserConstructionScript`
  (`parent.UserConstructionScript`))