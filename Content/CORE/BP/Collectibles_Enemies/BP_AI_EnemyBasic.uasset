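; BP_AI_EnemyBasic is a basic edible enemy that wanders at random and grants experience when eaten.
; From BeginPlay it loops a delay and an AIMoveTo to a random reachable point around itself, stopping with a debug print if the move fails.
; Eaten passes ExpPoint to BPCGetXP and destroys the actor, while capsule overlap only logs non-player actors.
; The construction script applies configurable speed and acceleration to CharacterMovement.
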(event OnComponentBeginOverlap(CapsuleComponent)
  (params (OverlappedComponent :type Primitive%20Component%20Object%20Reference) (OtherActor :type Actor%20Object%20Reference) (OtherComp :type Primitive%20Component%20Object%20Reference) (OtherBodyIndex :type Integer) (bFromSweep :type Boolean) (SweepResult :type Hit%20Result%20Structure%20%28by%20ref%29))
  ;[1 0.3603 0.3105 0.5] Detection
  (if (not (== OtherActor (CallFunction|GetPlayerOuroboros)))
    (Development|PrintString "NotPlayer")))

(event Custom|Random%20Roam
  ;[0.3326 0.9701 1 0.5] RandomMovement
  ;;[1 1 1 0.5] Delay D'apparition
  (Utilities|FlowControl|Delay (Variables|Default|GetApparitionDelay))
  (AI|AIMoveTo self (.RandomLocation (AI|Navigation|GetRandomReachablePointinRadius (Transformation|GetActorLocation) (Variables|Default|GetRadiusRangeOfMovement) 0 0)) 0 5.0 false
    (:OnSuccess
      (CallFunction|RandomRoam))
    (:OnFail
      (Development|PrintString "FailedAIPath"))))

(event EventBeginPlay
  (CallFunction|RandomRoam))

(event EventEaten
  ;[0.15 0 0.1437 0.5] Get Eaten
  (Default|Eaten (Variables|Default|GetBPC_GetXP) (Variables|Default|GetExpPoint))
  (Actor|DestroyActor))

(fn ConstructionScript
  (bind _charactermovement (Variables|Character|GetCharacterMovement))
  (Variables|/Script/Engine.CharacterMovementComponent|SetMaxWalkSpeed _charactermovement (Variables|Default|GetMax%20Walk%20Speed))
  (Variables|/Script/Engine.CharacterMovementComponent|SetMaxAcceleration _charactermovement (Variables|Default|GetMax%20Acceleration)))