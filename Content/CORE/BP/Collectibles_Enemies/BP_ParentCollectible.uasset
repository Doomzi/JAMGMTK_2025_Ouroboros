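; Parent Blueprint for collectibles and enemies in the Ouroboros game, handling contact damage, being eaten and distance culling.
; Its damage capsule hurts the player on contact with them or their bodies, then bounces away with a random turn and brief cooldown.
; Enemies drop spawn invincibility after a second and run a looping timer that despawns them when far, decrementing the GameMode count.
; GetEaten plays effects and destroys the actor, spawning a BP_Head for enemies.
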(event `self.ReceiveBeginPlay`
  (if (`self.Ennemies?`)
    (`KismetSystemLibrary.K2_SetTimerDelegate` (delegate `CheckDistanceWithPlayer`) 1.5 true)
    (`KismetSystemLibrary.Delay` 1.0)
    (set `self.InvincibilityOnSpawn` false)))

(event `CheckDistanceWithPlayer`
  (if (>= (`KismetMathLibrary.Vector_Distance` (`self.K2_GetActorLocation` (`/Game/CORE/FL_Macro.GetPlayerOuroboros`)) (`self.K2_GetActorLocation`)) (`self.MaxDistance`))
    (`self.DestroyEnnemyTooFar`)))

(event `self.DamageCapsule.OnComponentBeginOverlap`
  (params (OverlappedComponent :type "PrimitiveComponent Object Reference") (OtherActor :type "Actor Object Reference") (OtherComp :type "PrimitiveComponent Object Reference") (OtherBodyIndex :type Integer) (bFromSweep :type Boolean) (SweepResult :type "HitResult Structure (by ref)"))
  (bind (_returnvalue_x _returnvalue_y) (`KismetMathLibrary.BreakVector` (* (`KismetMathLibrary.Normal` (- (`self.K2_GetActorLocation`) (`self.K2_GetActorLocation` OtherActor))) 2000.0)))
  ;[1 0.3603 0.3105 0.5] Detection
  (if (not (`self.InvincibilityOnSpawn`))
    (if (`self.HasBounced?`)
      _
      (elif (== OtherActor (`/Game/CORE/FL_Macro.GetPlayerOuroboros`))
        (`GameplayStatics.ApplyDamage` (`/Game/CORE/FL_Macro.GetPlayerOuroboros`) (`self.Damage`) null self :!label _label)
        (`KismetSystemLibrary.PrintString` "PLAYER Hit")
        (`CharacterMovementComponent.AddImpulse` (`self.CharacterMovement`) (`KismetMathLibrary.MakeVector` _returnvalue_x _returnvalue_y) true)
        (`GameplayStatics.PlaySound2D` "/Game/CORE/Sound/SFX/SC_Bump.SC_Bump" 1.0 1.0 0.0 null null)
        (`SceneComponent.K2_AddWorldRotation` (`self.CapsuleComponent`) (`KismetMathLibrary.MakeRotator` 0.0 0.0 (`KismetMathLibrary.RandomFloatInRange` -60.0 60.0)) false false)
        (set `self.HasBounced?` true)
        (`KismetSystemLibrary.Delay` 0.5)
        (`MovementComponent.StopMovementImmediately` (`self.CharacterMovement`))
        (set `self.HasBounced?` false)
        (else
          (cast `/Game/CORE/BP/BP_Bodies` OtherActor
            (:`then`
              (goto _label))
            (:`CastFailed`
              (`KismetSystemLibrary.PrintString` (`KismetSystemLibrary.GetDisplayName` OtherActor)))))))
    (else
      (`KismetSystemLibrary.PrintString` "INVINCIBLE" true true (struct :`R` 1.0 :`G` 1.0 :`B` 1.0 :`A` 1.0)))))

(fn `DestroyEnnemyTooFar`
  (bind _asgame_mode_ouroboros (`/Game/CORE/FL_Macro.GetGameModeOuroboros`))
  (set `/Game/CORE/Game_Mode_Ouroboros.ActualNumberEnnemies` (- (`/Game/CORE/Game_Mode_Ouroboros.ActualNumberEnnemies` _asgame_mode_ouroboros) 1.0) _asgame_mode_ouroboros)
  (`self.K2_DestroyActor`))

(fn `GetEaten`
  (`NiagaraFunctionLibrary.SpawnSystemAtLocation` "/Game/CORE/VFX/NS_Kill_Enemy.NS_Kill_Enemy" (`self.K2_GetActorLocation`))
  (`GameplayStatics.PlaySound2D` "/Game/CORE/Sound/SFX/SC_EnemyExplose.SC_EnemyExplose" 1.0 1.0 0.0 null null)
  (if (`self.Ennemies?`)
    (`|SpawnActorFromClass` "/Game/CORE/BP/Collectibles_Enemies/BP_Head.BP_Head_C" (`KismetMathLibrary.MakeTransform` (`self.K2_GetActorLocation`)) "Undefined" "MultiplyWithRoot" null null))
  (`self.K2_DestroyActor`))

(fn `UserConstructionScript`)