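; Child enemy AI Blueprint that adds a random dash to the parent's roaming movement.
; Each roam rolls against RandomSpawnRate to run the parent roam or dash to a random reachable point with boosted speed, acceleration and range.
; Success restores speed and acceleration but leaves the dash range, as that variable is assigned to itself.
; Failure waits StunDuration, then roams again without restoring anything.
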(event `self.Event_RandomRoam`
  (bind _charactermovement (`self.CharacterMovement`))
  (bind _charactermovement_2 (`self.CharacterMovement`))
  (if (> (`KismetMathLibrary.RandomFloatInRange` 1.0 100.0) (`self.RandomSpawnRate`))
    ; Parent Movement Behavior
    (`parent.Event_RandomRoam`)
    (else
      (set `CharacterMovementComponent.MaxWalkSpeed` (`self.DashWalkSpeed`) _charactermovement_2)
      (set `CharacterMovementComponent.MaxAcceleration` (`self.DashAccelSpeed`) _charactermovement_2)
      (set `self.RadiusRangeOfMovement` (`self.DashRange`))
      (`|AIMoveTo` self (`NavigationSystemV1.K2_GetRandomReachablePointInRadius` (`self.K2_GetActorLocation`) (`self.RadiusRangeOfMovement`) null null) null
        (:`then`
          (`KismetSystemLibrary.PrintString` "Dash !!!"))
        (:`OnSuccess`
          (set `CharacterMovementComponent.MaxWalkSpeed` (`self.Max Walk Speed`) _charactermovement)
          (set `CharacterMovementComponent.MaxAcceleration` (`self.Max Acceleration`) _charactermovement)
          (set `self.RadiusRangeOfMovement` (`self.RadiusRangeOfMovement`))
          (`self.Event_RandomRoam`))
        (:`OnFail`
          (`KismetSystemLibrary.Delay` (`self.StunDuration`))
          (`self.Event_RandomRoam`))))))

(fn `UserConstructionScript`
  (`parent.UserConstructionScript`))