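; BP_Head is a short-lived physics head effect that pops into the air with a trail and sound, then vanishes.
; After a random delay, its Cube gets a randomized upward impulse and spins on Tick while a timeline updates its scale.
; When that timeline finishes, it spawns NB_Head and shortly destroys itself with a sound, before the delayed shrink-and-damping timeline can start.
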(event `self.ReceiveTick`
  (params (DeltaSeconds :type "Float (single-precision)"))
  (if (`self.Launched?`)
    (`SceneComponent.K2_AddWorldRotation` (`self.Cube`) (`KismetMathLibrary.MakeRotator` (`KismetMathLibrary.RandomFloatInRange` 3.0 6.0) (`KismetMathLibrary.RandomFloatInRange` 3.0 6.0)) false false)))

(event `self.ReceiveBeginPlay`
  (bind _cube (`self.Cube`))
  (bind _returnvalue (`SceneComponent.K2_GetComponentLocation` _cube))
  (bind _returnvalue_2 (`SceneComponent.K2_GetComponentRotation` _cube))
  (`|ExecutionSequence`
    (:`then_0`
      (`NiagaraFunctionLibrary.SpawnSystemAttached` "/Game/CORE/VFX/NS_Trail.NS_Trail" (`self.Cube`) "None" (0.0 0.0 0.0) (struct) "KeepRelativeOffset")
      (`GameplayStatics.PlaySound2D` "/Game/CORE/Sound/SFX/SC_HeadBop_Appear.SC_HeadBop_Appear" 1.0 1.0 0.0 null null))
    (:`then_1`
      (`KismetSystemLibrary.Delay` (`KismetMathLibrary.RandomFloatInRange` 0.0 0.5))
      (`PrimitiveComponent.AddImpulse` (`self.Cube`) (`KismetMathLibrary.MakeVector` (`KismetMathLibrary.RandomFloatInRange` -300.0 300.0) (`KismetMathLibrary.RandomFloatInRange` -300.0 300.0) (`KismetMathLibrary.RandomFloatInRange` 1200.0 1500.0)) "None" true)
      (set `self.Launched?` true)
      (`TimelineComponent.SetPlayRate` (`self.Timeline`) (/ 1.0 0.3))
      (bind _output_get (set `self.NewVar` (`KismetMathLibrary.RandomFloatInRange` 0.15 0.25)))
      (bind _output_get_2 (set `self.NewVar_0` (`KismetMathLibrary.RandomFloatInRange` 0.15 0.25)))
      (bind _output_get_3 (set `self.NewVar_1` (`KismetMathLibrary.RandomFloatInRange` 0.15 0.25)))
      (`Timeline|Timeline` :!via `PlayFromStart`
        (:`Update`
          (`SceneComponent.SetRelativeScale3D` (`self.Cube`) (`KismetMathLibrary.VLerp` (0.1 0.1 0.1) (`KismetMathLibrary.MakeVector` 0.0 _output_get _output_get_2) _output_get_3)))
        (:`Finished`
          (`|ExecutionSequence`
            (:`then_0`
              (`KismetSystemLibrary.Delay` 1.0)
              (`TimelineComponent.SetPlayRate` (`self.Timeline_0`) (/ 1.0 0.3))
              (bind (_direction _newtrack_0) (`Timeline|Timeline_0` :!via `PlayFromStart`)
                (:`Update`
                  (`SceneComponent.SetRelativeScale3D` (`self.Cube`) (`KismetMathLibrary.VLerp` (`KismetMathLibrary.MakeVector` (`self.NewVar`) (`self.NewVar_0`) (`self.NewVar_1`)) (0.01 0.01 0.01) _newtrack_0))
                  (`SceneComponent.K2_SetWorldLocationAndRotation` (stale _returnvalue_3) _returnvalue _returnvalue_2 false false)
                  (`PrimitiveComponent.SetLinearDamping` (`self.Cube`) (`KismetMathLibrary.Lerp` 0.1 1.0 _newtrack_0)))
                (:`Finished`
                  (bind _returnvalue_3 (`NiagaraFunctionLibrary.SpawnSystemAtLocation` "/Game/CORE/VFX/NB_Head.NB_Head" _returnvalue _returnvalue_2 :!label _label))
                  (`KismetSystemLibrary.Delay` 0.35)
                  (`GameplayStatics.PlaySound2D` "/Game/CORE/Sound/SFX/SC_HeadBop_Disapear.SC_HeadBop_Disapear" 1.0 1.0 0.0 null null)
                  (`self.K2_DestroyActor`))))
            (:`then_1`
              (goto _label))))))))

(fn `UserConstructionScript`)