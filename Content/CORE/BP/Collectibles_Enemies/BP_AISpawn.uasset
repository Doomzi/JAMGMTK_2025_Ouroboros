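; Enemy spawner actor that keeps spawning AI enemies inside its box volume, up to the game mode's map-wide cap.
; A self-restarting event waits a random delay divided by the combo-level multiplier, or an extra buffer at capacity.
; The player's level selects a DataTable row of weights for picking one of five enemy types.
; A line trace sets the spawn point, occasionally for a scattered group, where Basic replaces Big.
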(event `self.ReceiveBeginPlay`
  (`self.Event_SpawnAI`))

(event `Event_SpawnAI`
  (bind _asgame_mode_ouroboros (`/Game/CORE/FL_Macro.GetGameModeOuroboros`))
  (bind _asgame_mode_ouroboros_2 (`/Game/CORE/FL_Macro.GetGameModeOuroboros`))
  (bind _asgame_mode_ouroboros_3 (`/Game/CORE/FL_Macro.GetGameModeOuroboros`))
  (bind _box (`self.Box`))
  (bind (_returnvalue_x _returnvalue_y) (`KismetMathLibrary.BreakVector` (`KismetMathLibrary.RandomPointInBoundingBox` (`SceneComponent.K2_GetComponentLocation` _box) (`BoxComponent.BoxExtent` _box))))
  ;[0 0 0 0.5] SpawnRate
  (`KismetSystemLibrary.Delay` (/ (`KismetMathLibrary.RandomFloatInRange` (`self.MinSpawnMin`) (`self.MaxSpawnRate`)) (`BlueprintMapLibrary.Map_Find` (`/Game/CORE/Game_Mode_Ouroboros.ComboSpawnMultiplicator` _asgame_mode_ouroboros) (`/Game/CORE/Game_Mode_Ouroboros.ComboLevel` _asgame_mode_ouroboros))))
  (if (not (>= (`/Game/CORE/Game_Mode_Ouroboros.ActualNumberEnnemies` _asgame_mode_ouroboros_3) (`/Game/CORE/Game_Mode_Ouroboros.MaxEnnemiesInMap` _asgame_mode_ouroboros_3)))
    (bind _returnvalue (`|GetDataTableRow` "/Game/CORE/Data/Ouroboros_-_Spawn.Ouroboros_-_Spawn" (`KismetStringLibrary.Conv_StringToName` (`KismetStringLibrary.Conv_IntToString` (`KismetMathLibrary.Clamp` (`/Game/CORE/BP/BP_PlayerOuroboros.Level_Actual` (`/Game/CORE/FL_Macro.GetPlayerOuroboros`)) 0 31))))
      (:`then`
        (bind _indexthatwon (`self.DetermineIndex` (`KismetMathLibrary.RandomFloatInRange` 0.0 (`self.SumOfValues` _returnvalue))))
        (bind _outhit (`KismetSystemLibrary.LineTraceSingle` (`KismetMathLibrary.MakeVector` _returnvalue_x _returnvalue_y 2000.0) (`KismetMathLibrary.MakeVector` _returnvalue_x _returnvalue_y) "TraceTypeQuery1"))
        (if (`KismetMathLibrary.RandomBoolWithWeight` 0.2)
          (for _ (range (`KismetMathLibrary.RandomIntegerInRange` 2 4))
            (bind (_bblockinghit _binitialoverlap _time _distance _location _impactpoint) (`GameplayStatics.BreakHitResult` _outhit))
            (`|SpawnActorFromClass` (select `int` _indexthatwon :`0` "/Game/CORE/BP/Collectibles_Enemies/BP_AI_StaticEnemy.BP_AI_StaticEnemy_C" :`1` "/Game/CORE/BP/Collectibles_Enemies/BP_AI_BasicEnemy_Child.BP_AI_BasicEnemy_Child_C" :`2` "/Game/CORE/BP/Collectibles_Enemies/BP_AI_DashEnemy_Child.BP_AI_DashEnemy_Child_C" :`3` "/Game/CORE/BP/Collectibles_Enemies/BP_AI_ExplosiveEnemy_Child.BP_AI_ExplosiveEnemy_Child_C" :`4` "/Game/CORE/BP/Collectibles_Enemies/BP_AI_BasicEnemy_Child.BP_AI_BasicEnemy_Child_C" :!type "Actor Class Reference") (`KismetMathLibrary.MakeTransform` (`KismetMathLibrary.MakeVector` (+ (.x _impactpoint) (`KismetMathLibrary.RandomFloatInRange` -700.0 700.0)) (+ (.y _impactpoint) (`KismetMathLibrary.RandomFloatInRange` -700.0 700.0)) (+ (.z _impactpoint) 20.0)) (`KismetMathLibrary.RandomRotator` true)) "AdjustIfPossibleButAlwaysSpawn" "MultiplyWithRoot" null null)
            (set `/Game/CORE/Game_Mode_Ouroboros.ActualNumberEnnemies` (+ (`/Game/CORE/Game_Mode_Ouroboros.ActualNumberEnnemies` _asgame_mode_ouroboros_2) 1.0) _asgame_mode_ouroboros_2 :!label _label)
            (`self.Event_SpawnAI`))
          (else
            (`|SpawnActorFromClass` (select `int` _indexthatwon :`0` "/Game/CORE/BP/Collectibles_Enemies/BP_AI_StaticEnemy.BP_AI_StaticEnemy_C" :`1` "/Game/CORE/BP/Collectibles_Enemies/BP_AI_BasicEnemy_Child.BP_AI_BasicEnemy_Child_C" :`2` "/Game/CORE/BP/Collectibles_Enemies/BP_AI_DashEnemy_Child.BP_AI_DashEnemy_Child_C" :`3` "/Game/CORE/BP/Collectibles_Enemies/BP_AI_ExplosiveEnemy_Child.BP_AI_ExplosiveEnemy_Child_C" :`4` "/Game/CORE/BP/Collectibles_Enemies/BP_AI_BigEnemy.BP_AI_BigEnemy_C" :!type "Actor Class Reference") (`KismetMathLibrary.MakeTransform` (`KismetMathLibrary.MakeVector` (.x _impactpoint) (.y _impactpoint) (+ (.z _impactpoint) 20.0)) (`KismetMathLibrary.RandomRotator` true)) "AlwaysSpawn" "MultiplyWithRoot" null null)
            (goto _label)))))
    (else
      (`KismetSystemLibrary.Delay` (`self.MaxCapacityBuffer`))
      (`KismetSystemLibrary.PrintString` "MAX CAPACITY" true true (struct :`R` 1.0 :`G` 1.0 :`B` 1.0 :`A` 1.0))
      (`self.Event_SpawnAI`))))

(fn `DetermineIndex`
  (params (RandomValue :type "Float (double-precision)"))
  (returns (IndexThatWon :type Integer))
  (locals (LocalSum :type "Float (double-precision)"))
  (for (_array_element _array_index) (`self.WeightValues`)
    (bind _output_get (set `local.LocalSum` (+ _array_element (`local.LocalSum`))))
    (if (>= _output_get RandomValue)
      (break)))
  (return _array_index))

(fn `SumOfValues`
  (params (AllValues :type "/Game/CORE/Data/ST_SpawnRate Structure"))
  (returns (SomOfValues :type "Float (double-precision)"))
  (locals (LocalSum :type "Float (double-precision)"))
  (bind (_donottouch _static _normal _dash _bomb _big) (break `/Game/CORE/Data/ST_SpawnRate` AllValues))
  (bind _output_get (set `self.WeightValues` (`|MakeArray` (`KismetMathLibrary.Conv_IntToDouble` _static) (`KismetMathLibrary.Conv_IntToDouble` _normal) (`KismetMathLibrary.Conv_IntToDouble` _dash) (`KismetMathLibrary.Conv_IntToDouble` _bomb) (`KismetMathLibrary.Conv_IntToDouble` _big))))
  (for _array_element _output_get
    (set `local.LocalSum` (+ _array_element (`local.LocalSum`))))
  (return (`local.LocalSum`)))

(fn `UserConstructionScript`)