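; BP_AI_BasicEnemy is a basic enemy character that wanders randomly around the level.
; After a spawn delay it loops AI MoveTo to random reachable points within a radius of its current location, stopping with a debug print if a move fails.
; The construction script applies tunable walk speed and acceleration, and jumping is disabled.
; Capsule overlap detection is empty, and the obsolete get-eaten and XP logic is disconnected.
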(event `self.ReceiveBeginPlay`
  ;[1 1 1 0.5] Delay D'apparition
  (`KismetSystemLibrary.Delay` (`self.ApparitionDelay`))
  (`self.Event_RandomRoam`))

(event `Event_RandomRoam`
  ;[0.3326 0.9701 1 0.5] RandomMovement
  (`|AIMoveTo` self (`NavigationSystemV1.K2_GetRandomReachablePointInRadius` (`self.K2_GetActorLocation`) (`self.RadiusRangeOfMovement`) null null) null
    (:`OnSuccess`
      (`self.Event_RandomRoam`))
    (:`OnFail`
      (`KismetSystemLibrary.PrintString` "FailedAIPath"))))

(event `self.CapsuleComponent.OnComponentBeginOverlap`
  (params (OverlappedComponent :type "PrimitiveComponent Object Reference") (OtherActor :type "Actor Object Reference") (OtherComp :type "PrimitiveComponent Object Reference") (OtherBodyIndex :type Integer) (bFromSweep :type Boolean) (SweepResult :type "HitResult Structure (by ref)"))
  ;[1 0.3603 0.3105 0.5] Detection
)

(event `CustomEvent`
  ;[0.15 0 0.1437 0.5] Get Eaten (Obsolete)
)

(fn `CanJumpInternal`
  (returns (ReturnValue :type Boolean))
  (return false))

(fn `UserConstructionScript`
  (bind _charactermovement (`self.CharacterMovement`))
  (set `CharacterMovementComponent.MaxWalkSpeed` (`self.Max Walk Speed`) _charactermovement)
  (set `CharacterMovementComponent.MaxAcceleration` (`self.Max Acceleration`) _charactermovement)
  (`parent.UserConstructionScript`))