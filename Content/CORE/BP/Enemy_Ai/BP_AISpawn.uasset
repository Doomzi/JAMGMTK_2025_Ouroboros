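; Spawner actor that keeps producing BP_AI_EnemyBasic enemies inside its Box volume for as long as it runs.
; From BeginPlay, a self-calling event waits a random delay between MinSpawnMin and MaxSpawnRate, spawns one enemy, then repeats with no count limit.
; Spawn X and Y come from random points in the box, with collision adjustment.
; An unwired Select for choosing the enemy class remains unused.
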(event `self.ReceiveBeginPlay`
  (`self.Event_SpawnAI`))

(event `Event_SpawnAI`
  (bind _box (`self.Box`))
  (bind (_returnvalue_x _returnvalue_y) (`KismetMathLibrary.BreakVector` (`KismetMathLibrary.RandomPointInBoundingBox` (`SceneComponent.K2_GetComponentLocation` _box) (`BoxComponent.BoxExtent` _box))))
  ;[0 0 0 0.5] SpawnRate
  (`KismetSystemLibrary.Delay` (`KismetMathLibrary.RandomFloatInRange` (`self.MinSpawnMin`) (`self.MaxSpawnRate`)))
  (`|SpawnActorFromClass` "/Game/CORE/BP/Enemy_Ai/BP_AI_EnemyBasic.BP_AI_EnemyBasic_C" (`KismetMathLibrary.MakeTransform` (`KismetMathLibrary.MakeVector` _returnvalue_x _returnvalue_y)) "AdjustIfPossibleButDontSpawnIfColliding" "MultiplyWithRoot" null 0.0 0.0 0.0 0 0 0.2 null)
  (`self.Event_SpawnAI`))

(fn `UserConstructionScript`)