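; BP_Bodies is an actor for a decal-rendered body segment that can switch between body and tail forms.
; On BeginPlay it becomes a body, randomly picking the plain or animated body material and turning off the tail capsule's collision.
; TransformIntoTails swaps in the tail material and makes the tail capsule query-only, so collision queries detect only tail segments through that capsule.
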(event `self.ReceiveBeginPlay`
  (`self.TransformIntoBodies`))

(event `TransformIntoTails`
  (`DecalComponent.SetDecalMaterial` (`self.Decal`) (`self.MI_Tail`))
  (`PrimitiveComponent.SetCollisionEnabled` (`self.TailCapsule`) "QueryOnly"))

(event `TransformIntoBodies`
  (`DecalComponent.SetDecalMaterial` (`self.Decal`) (select `bool` (`KismetMathLibrary.RandomBool`) :`false` (`self.MI_Body`) :`true` (`self.MI_BodyAnim`)))
  (`PrimitiveComponent.SetCollisionEnabled` (`self.TailCapsule`) "NoCollision"))

(fn `UserConstructionScript`)