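; Player snake pawn that chases the cursor and eats collectibles by looping its head onto its tail.
; Body segments follow the head through an interpolated position history.
; Closing a loop briefly stops movement, grants invincibility, and ray-casts candidates against the body polygon, turning enclosed ones into XP and health.
; Data-table levels add segments and set speed and camera arm; border hits or depleted health reload the level.
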(event `LevelUP_Camera_Lenght`
  ; LevelUP_Camera_Lenght
  (`TimelineComponent.SetPlayRate` (`self.Timeline_Camera_ArmLenght`) (/ 1.0 0.5))
  (bind (_direction _newtrack_0) (`Timeline|Timeline_Camera_ArmLenght` :!via `PlayFromStart`)
    (:`Update`
      (bind _returnvalue (`|GetDataTableRow` "/Game/CORE/Data/DT_Player_Stats.DT_Player_Stats" (`KismetStringLibrary.Conv_StringToName` (`KismetStringLibrary.Conv_IntToString` (`self.Level_Actual`))))
        (:`then`
          (bind _returnvalue_2 (`|GetDataTableRow` "/Game/CORE/Data/DT_Player_Stats.DT_Player_Stats" (`KismetStringLibrary.Conv_StringToName` (`KismetStringLibrary.Conv_IntToString` (- (`self.Level_Actual`) 1))))
            (:`then`
              (bind _output_get (set `SpringArmComponent.TargetArmLength` (`KismetMathLibrary.Lerp` (`.Camera_TA_10_8BED84F14AB67F11AA52C28D320FFABC` (break `/Game/CORE/Data/ST_Level_Player` _returnvalue_2)) (`.Camera_TA_10_8BED84F14AB67F11AA52C28D320FFABC` (break `/Game/CORE/Data/ST_Level_Player` _returnvalue)) _newtrack_0) (`self.SpringArm`)))
              (set `self.TA_Lenght_Actual` _output_get))
            (:`RowNotFound`
              (`KismetSystemLibrary.PrintString` "ROW NOT FOUND 3"))))
        (:`RowNotFound`
          (`KismetSystemLibrary.PrintString` "ROW NOT FOUND 2"))))))

(event `self.ReceiveTick`
  (params (DeltaSeconds :type "Float (single-precision)"))
  (bind (_hitresult _returnvalue) (`PlayerController.GetHitResultUnderCursorByChannel` (`/Game/CORE/FL_Macro.GetPlayerControllerOuroboros`) "TraceTypeQuery1" true))
  (bind (_returnvalue_roll _returnvalue_pitch _returnvalue_yaw) (`KismetMathLibrary.BreakRotator` (`KismetMathLibrary.MakeRotFromX` (`self.Direction Player`))))
  (bind (_returnvalue_x _returnvalue_y _returnvalue_z) (`KismetMathLibrary.BreakVector` (* (`self.DeltaTime`) (* (`self.Direction Player`) (`self.Speed`)))))
  (set `self.DeltaTime` 0.0167)
  (`|ExecutionSequence`
    (:`then_0`
      ;[1 0.8189 0 0.5] Get CursorPosition
      (if _returnvalue
        (bind _output_get (set `self.CursorLocation` (`.Location` (`GameplayStatics.BreakHitResult` _hitresult))))
        ;[0.7708 0.03212 0.03212 0.5] CheckDistanceHeadAndCursor
        (if (< (`KismetMathLibrary.Vector_Distance` _output_get (`self.K2_GetActorLocation`)) 150.0)
          (set `self.CursorNearHead?` true)
          (else
            (set `self.CursorNearHead?` false)))))
    (:`then_1`
      ;[0.1765 0.7865 0 0.5] Setup For Body movement
      (set `self.DeplacementParFrame` (* (`self.Speed`) (`self.DeltaTime`)))
      (set `self.FrameSpaceBetweenBodies` (/ (`self.SpaceBetweenBodies`) (`self.DeplacementParFrame`)))
      (set `self.MaxPositionHistoryLenght` (+ (`KismetMathLibrary.FFloor` (* (`self.FrameSpaceBetweenBodies`) (`self.BodyCount`))) 2))
      ;[0.1765 0.7865 0 0.5] Move player to cursor
      (if (not (`self.CursorNearHead?`))
        (set `self.Direction Player` (`KismetMathLibrary.Normal` (- (`self.CursorLocation`) (`self.K2_GetActorLocation`)))))
      (if (not (`self.StopMovement`))
        (`self.K2_AddActorWorldOffset` (`KismetMathLibrary.MakeVector` _returnvalue_x _returnvalue_y _returnvalue_z))
        (`self.K2_SetActorRotation` (`KismetMathLibrary.MakeRotator` 0.0 0.0 _returnvalue_yaw))
        ;[0.1765 0.7865 0 0.5] Movement Lerp Logic (Bodies)
        ;; Store all position (Player)
        (`KismetArrayLibrary.Array_Insert` (`self.PositionHistory`) (`self.K2_GetActorLocation`))
        (`|ExecutionSequence`
          (:`then_0`
            ;; If Position History is greater than (Max Position) remove the last index
            (if (> (`KismetArrayLibrary.Array_Length` (`self.PositionHistory`)) (`self.MaxPositionHistoryLenght`))
              (`KismetArrayLibrary.Array_Remove` (`self.PositionHistory`) (- (`KismetArrayLibrary.Array_Length` (`self.PositionHistory`)) 1))))
          (:`then_1`
            ;; Lerp all bodies and tails compare to location (Position History)
            (for _index (range (`self.BodyCount`))
              (set `self.FrameDelay` (`KismetMathLibrary.FFloor` (* (`KismetMathLibrary.Conv_IntToDouble` (+ _index 1)) (/ (`self.SpaceBetweenBodies`) (`self.DeplacementParFrame`)))))
              (bind _output (`|GetArrayItem` (`self.BodiesArray`) _index))
              (`self.K2_SetActorLocation` _output (`KismetMathLibrary.VInterpTo` (`self.K2_GetActorLocation` _output) (`|GetArrayItem` (`self.PositionHistory`) (`self.FrameDelay`)) (`self.DeltaTime`) 25.0) false false)
              ;; Lerp bodies rotation
              (bind _output_get_2 (set `self.DirectionForBodies(Rotation)` (`KismetMathLibrary.Normal` (- (`|GetArrayItem` (`self.PositionHistory`) (- (`self.FrameDelay`) 1)) (`self.K2_GetActorLocation` _output)))))
              (bind (_returnvalue_roll_2 _returnvalue_pitch_2 _returnvalue_yaw_2) (`KismetMathLibrary.BreakRotator` (`KismetMathLibrary.MakeRotFromX` _output_get_2)))
              (`self.K2_SetActorRotation` _output (`KismetMathLibrary.MakeRotator` 0.0 0.0 _returnvalue_yaw_2) false))))))))

(event `self.ReceiveBeginPlay`
  ; Begin Play
  (bind _returnvalue (`|GetDataTableRow` "/Game/CORE/Data/DT_Player_Stats.DT_Player_Stats" (`KismetStringLibrary.Conv_StringToName` (`KismetStringLibrary.Conv_IntToString` (`self.Level_Actual`))))
    (:`then`
      (set `self.Health` (`.Health_14_28C0134C444702E3E5873587690076D2` (break `/Game/CORE/Data/ST_Level_Player` _returnvalue)))
      (set `SpringArmComponent.TargetArmLength` (`.Camera_TA_10_8BED84F14AB67F11AA52C28D320FFABC` (break `/Game/CORE/Data/ST_Level_Player` _returnvalue)) (`self.SpringArm`))
      (set `self.XP_Max_Level-Actual` (`.XP_Max_7_5532B034440A00D011B5C59298C27D10` (break `/Game/CORE/Data/ST_Level_Player` _returnvalue)))
      (set `self.Speed` (`.Speed_19_DD144D0543353914D3FE29954719065C` (break `/Game/CORE/Data/ST_Level_Player` _returnvalue)))
      (bind _returnvalue_2 (`|CreateWidget` "/Game/CORE/UI/HUD/WBP_HUD.WBP_HUD_C"))
      (`UserWidget.AddToViewport` _returnvalue_2 0)
      (set `self.HUD` _returnvalue_2))))

(event `self.HeadCollision.OnComponentBeginOverlap`
  (params (OverlappedComponent :type "PrimitiveComponent Object Reference") (OtherActor :type "Actor Object Reference") (OtherComp :type "PrimitiveComponent Object Reference") (OtherBodyIndex :type Integer) (bFromSweep :type Boolean) (SweepResult :type "HitResult Structure (by ref)"))
  ;[0.7708 0.03212 0.03212 0.5] CheckDistance Head with tails (Trigger Eat action)
  (if (== OtherActor (`self.ActualTail`))
    (set `self.ShapeClosed?` true)
    (if (not (`self.InvincibilityShapeClosed`))
      (`self.StartCheckIfInCircle`)
      (`self.CE_StopMovement` true))
    (else
      (set `self.ShapeClosed?` false)
      (cast `/Game/CORE/BP/LD/BP_Bordure` OtherActor)
      (`self.DieFunction`))))

(event `CE_StopMovement`
  (params (StopMovement :type Boolean))
  ; Stopmovement
  (set `self.StopMovement` StopMovement)
  (`KismetSystemLibrary.Delay` 0.3)
  (set `self.StopMovement` false)
  (`self.ResetCircleCalculation`)
  (set `self.ShapeClosed?` false))

(event `Key|P`
  (params (Key :type "Key Structure"))
  ;[0.7792 0 1 0.5] BUTTON TEST
  (:`Pressed`
    (`self.AddNewBodyToSnake`)))

(event `self.HeadCollisionForBodies.OnComponentBeginOverlap`
  (params (OverlappedComponent :type "PrimitiveComponent Object Reference") (OtherActor :type "Actor Object Reference") (OtherComp :type "PrimitiveComponent Object Reference") (OtherBodyIndex :type Integer) (bFromSweep :type Boolean) (SweepResult :type "HitResult Structure (by ref)"))
  (bind _bodiesarray (`self.BodiesArray`))
  ; Detect and damage self collision
  (bind _asbp_bodies (cast `/Game/CORE/BP/BP_Bodies` OtherActor))
  (if (or (== _asbp_bodies (`|GetArrayItem` (`self.BodiesArray`))) (== _asbp_bodies (`|GetArrayItem` (`self.BodiesArray`) 1)) (== _asbp_bodies (`|GetArrayItem` _bodiesarray (`KismetArrayLibrary.Array_LastIndex` _bodiesarray))))
    _
    (elif (not (`self.InvincibilityHited`))
      (`GameplayStatics.ApplyDamage` self (`/Game/CORE/BP/BP_Bodies.DamageToSnake` _asbp_bodies)))))

(event `Key|E`
  (params (Key :type "Key Structure"))
  ;[0.7792 0 1 0.5] BUTTON TEST
)

(event `SetNewTailOnlyForStart`
  ; SetNewTailOnlyForStart
  (`KismetSystemLibrary.Delay` 0.2)
  (`/Game/CORE/BP/BP_Bodies.TransformIntoTails` (`self.ActualTail`)))

(event `self.ReceiveAnyDamage`
  (params (Damage :type "Float (single-precision)") (DamageType :type "DamageType Object Reference") (InstigatedBy :type "Controller Object Reference") (DamageCauser :type "Actor Object Reference"))
  ; Take damage
  (`self.Damage` Damage DamageCauser))

(event `StartCheckIfInCircle`
  ;[0.7708 0.03212 0.03212 0.5] CheckIfSomething is in the shape
  (`KismetArrayLibrary.Array_Clear` (`self.PolygonVector`))
  (`self.ResetCircleCalculation`)
  (`self.SetInvinciblityShapeClosed` true)
  (`self.TriggerInvincibilityHited`)
  ;; Setup and save actual position of snake
  (for _index (range (`KismetArrayLibrary.Array_Length` (`self.BodiesArray`)))
    (`KismetArrayLibrary.Array_Add` (`self.PolygonVector`) (`self.K2_GetActorLocation` (`|GetArrayItem` (`self.BodiesArray`) _index))))
  (`self.RelaunchCheckCollectibleInTheCircle`))

(event `RelaunchCheckCollectibleInTheCircle`
  (bind _collectibleinsidethecollision (`self.CollectibleInsideTheCollision`))
  (bind _collectibleinsidethecollision_2 (`self.CollectibleInsideTheCollision`))
  (bind _collectiblecheckrduringoneshape (`self.CollectibleCheckrDuringOneShape`))
  (bind _croisementcount (`self.CroisementCount`))
  (bind _playertest (`self.PlayerTest`))
  (bind _returnvalue (`KismetMathLibrary.FTrunc` _collectiblecheckrduringoneshape))
  (bind _returnvalue_x (`KismetMathLibrary.BreakVector` (`self.K2_GetActorLocation` (`self.PlayerTest`))))
  (bind (_returnvalue_x_2 _returnvalue_y) (`KismetMathLibrary.BreakVector` (`self.K2_GetActorLocation` (`self.PlayerTest`))))
  (bind (_returnvalue_x_3 _returnvalue_y_2) (`KismetMathLibrary.BreakVector` (`self.K2_GetActorLocation` (`self.PlayerTest`))))
  (bind (_returnvalue_x_4 _returnvalue_y_3) (`KismetMathLibrary.BreakVector` (`self.K2_GetActorLocation` (`self.PlayerTest`))))
  (bind _returnvalue_2 (mod _croisementcount 2))
  (bind (_output_x _output_y) (`KismetMathLibrary.BreakVector` (`|GetArrayItem` (`self.PolygonVector`) (`self.A`))))
  (bind (_output_x_2 _output_y_2) (`KismetMathLibrary.BreakVector` (`|GetArrayItem` (`self.PolygonVector`) (`self.B`))))
  (bind _output_x_3 (`KismetMathLibrary.BreakVector` (`|GetArrayItem` (`self.PolygonVector`) (`self.A`))))
  (bind (_output_x_4 _output_y_3) (`KismetMathLibrary.BreakVector` (`|GetArrayItem` (`self.PolygonVector`) (`self.A`))))
  (bind (_output_x_5 _output_y_4) (`KismetMathLibrary.BreakVector` (`|GetArrayItem` (`self.PolygonVector`) (`self.A`))))
  (bind _output (`|GetArrayItem` _collectibleinsidethecollision_2 _returnvalue))
  ;[0.7708 0.03212 0.03212 0.5] CheckIfSomething is in the shape
  (if (>= _collectiblecheckrduringoneshape (`KismetArrayLibrary.Array_Length` (`self.CollectibleInsideTheCollision`)))
    (set `self.ShapeClosed?` false)
    (set `self.CollectibleCheckrDuringOneShape` 0.0)
    (`self.ResetCircleCalculation`)
    (`self.EatAllCollectibles`)
    (`self.TestRemoveInvincibility`)
    (else
      (`/Engine/EditorBlueprintResources/StandardMacros.IsValid` _output
        (:`Is Valid`
          (bind _output_get (set `self.PlayerTest` _output))
          (`KismetSystemLibrary.PrintString` (`KismetSystemLibrary.GetDisplayName` _output_get))
          (`self.ResetCircleCalculation`)
          (for _index (range (`KismetArrayLibrary.Array_Length` (`self.PolygonVector`)))
            (set `self.A` _index)
            (bind _returnvalue_3 (`KismetMathLibrary.Conv_IntToDouble` (+ _index 1)))
            (set `self.B` (`KismetMathLibrary.FTrunc` (`KismetMathLibrary.SelectFloat` (mod _returnvalue_3 (`KismetMathLibrary.Conv_IntToDouble` (`KismetArrayLibrary.Array_Length` (`self.PolygonVector`)))) _returnvalue_3 (`self.ShapeClosed?`))))
            (set `self.B/Y` _output_y_2)
            (bind _output_get_2 (set `self.B/X` _output_x_2))
            (if (!= (> (`self.B/Y`) _returnvalue_y_3) (> _output_y _returnvalue_y))
              (if (< _returnvalue_x (+ (/ (* (- (`self.B/X`) _output_x_4) (- _returnvalue_y_2 _output_y_3)) (- (`self.B/Y`) _output_y_4)) _output_x_3))
                (if (`self.ShapeClosed?`)
                  (`/Engine/EditorBlueprintResources/StandardMacros.IncrementInt` (`self.CroisementCount`))))))
          (if (== _croisementcount 0)
            (`/Engine/EditorBlueprintResources/StandardMacros.IncrementFloat` (`self.CollectibleCheckrDuringOneShape`)
              (:`  `
                (`self.RelaunchCheckCollectibleInTheCircle`)))
            (else
              (if (== _returnvalue_2 1)
                (`KismetSystemLibrary.PrintString` (`KismetStringLibrary.Concat_StrStr` "INSIDE : " (`KismetStringLibrary.Conv_IntToString` _returnvalue_2) "NB croisement : " (`KismetStringLibrary.Conv_IntToString` _croisementcount)) true true (struct :`R` 1.0 :`B` 0.114047 :`A` 1.0) 5.0)
                (`KismetArrayLibrary.Array_Remove` _collectibleinsidethecollision (`KismetArrayLibrary.Array_Find` _collectibleinsidethecollision _playertest))
                (`KismetArrayLibrary.Array_Add` (`self.EatenCollectibles`) _playertest)
                (else
                  (`/Engine/EditorBlueprintResources/StandardMacros.IncrementFloat` (`self.CollectibleCheckrDuringOneShape`)
                    (:`  `
                      _))))
              (`self.RelaunchCheckCollectibleInTheCircle`))))
        (:`Is Not Valid`
          (`KismetArrayLibrary.Array_Remove` _collectibleinsidethecollision_2 _returnvalue)
          (`self.RelaunchCheckCollectibleInTheCircle`))))))

(event `TestRemoveInvincibility`
  ; TestRemoveInvinci A CHANGER
  (`KismetSystemLibrary.Delay` (`self.TimeInvincibilityShapeClosed`))
  (`self.SetInvinciblityShapeClosed` false))

(event `TriggerInvincibilityHited`
  ; Trigger invicibility Hited
  (set `self.InvincibilityHited` true)
  (`KismetSystemLibrary.Delay` (`self.TimeInvinciblityHited`))
  (set `self.InvincibilityHited` false))

(event `ResetCircleCalculation`
  ;[0.7708 0.03212 0.03212 0.5] CheckIfSomething is in the shape
  ;; Reset variable after a circle
  (set `self.CroisementCount` 0))

(event `self.CollisionDetectShape.OnComponentBeginOverlap`
  (params (OverlappedComponent :type "PrimitiveComponent Object Reference") (OtherActor :type "Actor Object Reference") (OtherComp :type "PrimitiveComponent Object Reference") (OtherBodyIndex :type Integer) (bFromSweep :type Boolean) (SweepResult :type "HitResult Structure (by ref)"))
  (bind _asbp_parent_collectible (cast `/Game/CORE/BP/Collectibles_Enemies/BP_ParentCollectible` OtherActor))
  (`KismetArrayLibrary.Array_Add` (`self.CollectibleInsideTheCollision`) _asbp_parent_collectible))

(event `self.CollisionDetectShape.OnComponentEndOverlap`
  (params (OverlappedComponent :type "PrimitiveComponent Object Reference") (OtherActor :type "Actor Object Reference") (OtherComp :type "PrimitiveComponent Object Reference") (OtherBodyIndex :type Integer))
  (bind _collectibleinsidethecollision (`self.CollectibleInsideTheCollision`))
  (bind _asbp_parent_collectible (cast `/Game/CORE/BP/Collectibles_Enemies/BP_ParentCollectible` OtherActor))
  (if (`KismetArrayLibrary.Array_Contains` _collectibleinsidethecollision _asbp_parent_collectible)
    (`KismetArrayLibrary.Array_RemoveItem` _collectibleinsidethecollision _asbp_parent_collectible)))

(fn `AddNewBodyToSnake`
  (bind _bodiesarray (`self.BodiesArray`))
  (bind _output (`|GetArrayItem` _bodiesarray (`KismetArrayLibrary.Array_LastIndex` _bodiesarray)))
  (`/Game/CORE/BP/BP_Bodies.TransformIntoBodies` (`self.ActualTail`))
  (bind _returnvalue (`AddComponent|NODE_AddChildActorComponent-1`))
  (bind _asbp_bodies (cast `/Game/CORE/BP/BP_Bodies` (`ChildActorComponent.ChildActor` _returnvalue)))
  (`KismetArrayLibrary.Array_Add` (`self.BodiesArray`) _asbp_bodies)
  (`SceneComponent.K2_DetachFromComponent` _returnvalue "KeepRelative" "KeepRelative" "KeepRelative" true)
  (`/Engine/EditorBlueprintResources/StandardMacros.IncrementInt` (`self.BodyCount`)
    (:`  `
      (`/Game/CORE/BP/BP_Bodies.TransformIntoTails` _output)
      (set `self.ActualTail` _output))))

(fn `Damage`
  (params (DamageTaken :type "Float (double-precision)") (`Damage Causer` :type "Actor Object Reference"))
  (`self.TriggerInvincibilityHited`)
  (set `self.Damage Causer` `Damage Causer`)
  (bind _output_get (set `self.Health` (- (`self.Health`) DamageTaken)))
  (`KismetSystemLibrary.PrintString` (`KismetStringLibrary.Concat_StrStr` "Health : " (`KismetStringLibrary.Conv_DoubleToString` _output_get)))
  (`/Game/CORE/UI/HUD/WBP_HUD.Set_HP_HUD` (`self.HUD`) (`self.Health`) (`self.MaxHealth`) true)
  (if (<= (`self.Health`) 0.0)
    (`self.DieFunction`)))

(fn `DieFunction`
  (`KismetSystemLibrary.PrintString` "DIE")
  (bind _returnvalue (`GameplayStatics.GetCurrentLevelName` true))
  (`GameplayStatics.OpenLevel` (`KismetStringLibrary.Conv_StringToName` _returnvalue)))

(fn `EatAllCollectibles`
  (for _array_element (`self.EatenCollectibles`)
    (`KismetSystemLibrary.PrintString` (`KismetSystemLibrary.GetDisplayName` _array_element) true true (struct :`R` 0.770833 :`G` 0.032118 :`B` 0.032118 :`A` 0.5))
    (bind _output_get (set `self.XP_Earned` (`KismetMathLibrary.FTrunc` (`/Game/CORE/BP/Collectibles_Enemies/BP_ParentCollectible.ExpPoint` _array_element))))
    (`self.GainXP` _output_get)
    (`/Game/CORE/BP/Collectibles_Enemies/BP_ParentCollectible.GetEaten` _array_element)
    (`self.GainLife` 2.0)
    (`KismetArrayLibrary.Array_RemoveItem` (`self.EatenCollectibles`) _array_element))
  (`KismetArrayLibrary.Array_Clear` (`self.EatenCollectibles`)))

(fn `GainLife`
  (params (LifePoint :type "Float (double-precision)"))
  (bind _output_get (set `self.Health` (+ LifePoint (`self.Health`))))
  (`KismetSystemLibrary.PrintString` (`KismetStringLibrary.Concat_StrStr` "Health : " (`KismetStringLibrary.Conv_DoubleToString` _output_get))))

(fn `GainXP`
  (params (XP_Earned :type Integer))
  (bind _returnvalue (>= (`self.XP_Current`) (`self.XP_Max_Level-Actual`)))
  (set `self.XP_Current` (+ XP_Earned (`self.XP_Current`)))
  (bind (_level __health __xp_max __body_count_max __camera_ta __speed __text) (`self.GetPlayerStats` (`self.Level_Actual`)))
  (set `self.XP_Max_Level-Actual` __xp_max)
  (set `self.TextLevel` __text)
  (bind (_level_2 __health_2 __xp_max_2) (`self.GetPlayerStats` (`KismetMathLibrary.Clamp` (- (`self.Level_Actual`) 1) 0 99999999)))
  (set `self.Previous Level Max` __xp_max_2)
  (`/Game/CORE/UI/HUD/WBP_HUD.Set_XP_HUD` (`self.HUD`) (`self.TextLevel`) (`KismetMathLibrary.Conv_IntToDouble` (`self.XP_Current`)) (`KismetMathLibrary.Conv_IntToDouble` (`self.XP_Max_Level-Actual`)) (`KismetMathLibrary.Conv_IntToDouble` (`self.Previous Level Max`)) false _returnvalue (`self.Level_Actual`))
  (if _returnvalue
    (`self.LevelUp`)))

(fn `GetPlayerStats`
  (params (Level_Select :type Integer))
  (returns (Level :type Integer) (` Health` :type "Float (double-precision)") (` XP Max` :type Integer) (` Body Count Max` :type Integer) (` Camera TA` :type "Float (double-precision)") (` Speed` :type "Float (double-precision)") (` Text` :type Text))
  (bind _returnvalue (`|GetDataTableRow` "/Game/CORE/Data/DT_Player_Stats.DT_Player_Stats" (`KismetStringLibrary.Conv_StringToName` (`KismetStringLibrary.Conv_IntToString` Level_Select)))
    (:`then`
      (bind _output_get (set `self.ActualStats` _returnvalue))
      (return Level_Select (`.Health_14_28C0134C444702E3E5873587690076D2` (break `/Game/CORE/Data/ST_Level_Player` _output_get)) (`.XP_Max_7_5532B034440A00D011B5C59298C27D10` (break `/Game/CORE/Data/ST_Level_Player` _output_get)) (`.Body_Count_Max_8_FD3CB5AB4D9A76D0897EC9A6947C9DA4` (break `/Game/CORE/Data/ST_Level_Player` _output_get)) (`.Camera_TA_10_8BED84F14AB67F11AA52C28D320FFABC` (break `/Game/CORE/Data/ST_Level_Player` _output_get)) (`.Speed_19_DD144D0543353914D3FE29954719065C` (break `/Game/CORE/Data/ST_Level_Player` _output_get)) (`.Text_22_4533A273421887014FA8DAB22E4E759C` (break `/Game/CORE/Data/ST_Level_Player` _output_get))))))

(fn `LevelUp`
  (set `self.Previous Level Max` (`self.XP_Max_Level-Actual`))
  (bind _result (`/Engine/EditorBlueprintResources/StandardMacros.IncrementInt` (`self.Level_Actual`))
    (:`  `
      (`self.AddNewBodyToSnake`)
      (`self.LevelUP_Camera_Lenght`)
      (bind (_level __health __xp_max __body_count_max __camera_ta __speed) (`self.GetPlayerStats` (`self.Level_Actual`)))
      (set `self.Speed` __speed)
      (set `self.MaxHealth` __health)
      (set `self.XP_Max_Level-Actual` __xp_max)
      (`/Game/CORE/UI/HUD/WBP_HUD.Set_HP_Max` (`self.HUD`) 1.0)
      (`/Game/CORE/UI/HUD/WBP_HUD.Set_XP_HUD` (`self.HUD`) "" (`KismetMathLibrary.Conv_IntToDouble` (`self.XP_Current`)) (`KismetMathLibrary.Conv_IntToDouble` (`self.XP_Max_Level-Actual`)) (`KismetMathLibrary.Conv_IntToDouble` (`self.Previous Level Max`)) false false (`self.Level_Actual`))
      (`KismetSystemLibrary.PrintString` (`KismetStringLibrary.Conv_DoubleToString` (`self.Speed`)) true true (struct :`R` 0.08142 :`G` 1.0 :`A` 1.0)))))

(fn `SetBodiesOnStart`
  (bind _bodiesarray (`self.BodiesArray`))
  (for _array_element (`self.BodiesArray`)
    (`self.K2_DestroyActor` _array_element))
  (`KismetArrayLibrary.Array_Clear` (`self.BodiesArray`))
  (for _index (range (`self.BodyCount`))
    (bind _returnvalue (`AddComponent|NODE_AddChildActorComponent-0`))
    (bind _asbp_bodies (cast `/Game/CORE/BP/BP_Bodies` (`ChildActorComponent.ChildActor` _returnvalue)))
    (`KismetArrayLibrary.Array_Add` (`self.BodiesArray`) _asbp_bodies)
    (`SceneComponent.K2_DetachFromComponent` _returnvalue "KeepRelative" "KeepRelative" "KeepRelative" true)
    (if (== (- (`self.BodyCount`) 1) _index)
      _))
  (set `self.ActualTail` (`|GetArrayItem` _bodiesarray (`KismetArrayLibrary.Array_LastIndex` _bodiesarray)))
  (`SphereComponent.SetSphereRadius` (`self.CollisionDetectShape`) (`KismetMathLibrary.Conv_IntToDouble` (* (+ (`self.BodyCount`) 1) 250)) true)
  (`self.SetNewTailOnlyForStart`))

(fn `SetInvinciblityShapeClosed`
  (params (Invincibility :type Boolean))
  (set `self.InvincibilityShapeClosed` Invincibility))

(fn `UserConstructionScript`
  (`self.SetBodiesOnStart`))